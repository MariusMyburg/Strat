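; Base Blueprint for player ships, providing movement requests that spend movement points and a getter for the ship's crew component.
; Forward moves nudge the root along its facing without sweep, turns rotate it in 90-degree steps, and each subtracts the movement cost without checking the remaining points.
; Tick currently drives the ship automatically, moving forward every frame and turning left after a repeating five-second Delay.
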(event EventBeginPlay)

(event Collision|EventActorBeginOverlap
  (params (OtherActor :type Actor%20Object%20Reference)))

(event EventMoveForward
  ;[1 1 1] Base Ship Forward Movement Request Handling
  (Transformation|SetWorldLocation (Variables|Default|GetDefaultSceneRoot) (+ (Transformation|GetWorldLocation (Variables|Default|GetDefaultSceneRoot)) (* (Math|Vector|GetForwardVector (Transformation|GetWorldRotation (Variables|Default|GetDefaultSceneRoot))) 0.8)) false false)
  ;[1 1 1] Update movement points based on cost
  (Variables|Ship|SetMovementPoints (- (Variables|Ship|GetMovementPoints) (Variables|ShipAdvanced|GetMovementPointCost))))

(event EventTick
  (params (DeltaSeconds :type Float%20%28single-precision%29))
  (CallFunction|MoveForward)
  (Utilities|FlowControl|Delay 5.0)
  (CallFunction|TurnLeft))

(event EventTurnLeft
  ;[1 1 1] Base Ship Turn Left Movement Request Handling
  (Transformation|AddLocalRotation (Variables|Default|GetDefaultSceneRoot) "90.000000, 0, 0" false false)
  ;[1 1 1] Update movement points based on cost
  (Variables|Ship|SetMovementPoints (- (Variables|Ship|GetMovementPoints) (Variables|ShipAdvanced|GetMovementPointCost))))

(event EventTurnRight
  ;[1 1 1] Base Ship Turn Right Movement Request Handling
  (Transformation|AddLocalRotation (Variables|Default|GetDefaultSceneRoot) "-90.000000, 0, 0" false false)
  ;[1 1 1] Update movement points based on cost
  (Variables|Ship|SetMovementPoints (- (Variables|Ship|GetMovementPoints) (Variables|ShipAdvanced|GetMovementPointCost))))

(fn ConstructionScript)

(fn GetCrew
  ;[1 1 1] Every PlayerShip has a Crew
  (return (Variables|Default|GetBP_CrewComponent)))