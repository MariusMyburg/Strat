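; BP_CrewComponent is a crew roster component that stores crew member objects for the strategy game.
; AddCrewMember has BP_StratGameMode create a new crew member object, names it after the Class input, inserts it at the front of CrewMemberInfos and prints the crew count.
; The skill inputs (Leadership, Piloting, Gunnery, Mechanics, Hacking) feed only an unused struct node, so they are not applied to the new member.
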(event EventBeginPlay)

(event EventTick
  (params (DeltaSeconds :type Float%20%28single-precision%29)))

(fn AddCrewMember
  (params (Class :type String) (Leadership :type Float%20%28single-precision%29) (Piloting :type Float%20%28single-precision%29) (Gunnery :type Float%20%28single-precision%29) (Mechanics :type Float%20%28single-precision%29) (Hacking :type Float%20%28single-precision%29))
  (bind _asbp_strat_game_mode (Utilities|Casting|CastToBP_StratGameMode (Game|GetGameMode)))
  (bind _createdcrewmemberobject (Default|CreateNewCrewMemberObject _asbp_strat_game_mode))
  (bind _output_get (LocalVariables|SetNewCrewMember _createdcrewmemberobject))
  (Variables|/Game/Blueprints/Crew/BP_CrewMember.BP_CrewMember_C|SetName _output_get Class)
  (Utilities|Array|Insert (Variables|Default|GetCrewMemberInfos) _output_get)
  (Development|PrintString (Utilities|String|Append "We now have " (Utilities|String|ToString(Integer) (Utilities|Array|Length (Variables|Default|GetCrewMemberInfos))) " crew members.")))