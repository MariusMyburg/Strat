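; BP_StratGameInstance is the game instance for a ship-based strategy game, holding turn and combat state.
; EvaluateGameState scans player ships for the highest LastActionTime, assigning CurrentTurn only while it is unset.
; SetLastMoved records the last ship and, when its movement and action points run out, only prints a turn-switch TODO.
; Helpers open a combat level with its widget and draw a debug line from the player pawn.
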(event EventEvaluateGameState
  (bind _outactors (Actor|GetAllActorsOfClass "/Game/Blueprints/Player/BP_PlayerShipBase.BP_PlayerShipBase_C"))
  (Utilities|FlowControl|Sequence
    (:then_0
      (for _array_element _outactors
        (if (>= (Variables|/Game/Blueprints/Player/BP_PlayerShipBase.BP_PlayerShipBase_C|GetLastActionTime _array_element) (Variables|Default|GetMaxLastActionTime))
          (Variables|Default|SetMaxLastActionTime (Variables|/Game/Blueprints/Player/BP_PlayerShipBase.BP_PlayerShipBase_C|GetLastActionTime _array_element))
          (Utilities|IsValid (Variables|Default|GetCurrentTurn)
            (:Is%20Not%20Valid
              (Variables|Default|SetCurrentTurn _array_element))))))))

(fn StartCombatMode
  (params (Level :type String))
  (Game|OpenLevel(byName) (Utilities|String|StringToName Level))
  (bind _returnvalue (UserInterface|CreateWidget "/Game/UI/BP_CombatWidget.BP_CombatWidget_C"))
  (UserInterface|Viewport|AddtoViewport _returnvalue 0))

(fn DrawTacticalOverlay
  (bind _returnvalue (Game|Player|GetPlayerPawn 0))
  (Utilities|IsValid _returnvalue
    (:Is%20Valid
      (Rendering|Debug|DrawDebugLine (Transformation|GetActorLocation _returnvalue) "0, 0, 0" "(R=1.000000,G=0.214129,B=0.000000,A=1.000000)" 0.0 1e+01))))

(fn SetLastMoved
  (params (Ship :type BP%20Player%20Ship%20Base%20Object%20Reference))
  (bind _output_get (Variables|Default|SetLastMoved Ship))
  (if (<= (+ (Variables|/Game/Blueprints/Player/BP_PlayerShipBase.BP_PlayerShipBase_C|GetMovementPoints _output_get) (Variables|/Game/Blueprints/Player/BP_PlayerShipBase.BP_PlayerShipBase_C|GetActionPoints _output_get)) 0.0)
    (Development|PrintString "OTHER PLAYER TURN: TODO SWITCH PLAYER")))